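; Button Blueprint that spawns a random batch of UFOs when pressed.
; It extends a parent button's press event, then spawns two to five BP_UFO actors at random points around its Box component.
; Spawn points come from a bounding box at the Box's world location, using its scaled extent vector rotated by the component's world rotation.
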(event EventButtonPressed
  (bind _box (Variables|Default|GetBox))
  ;[1 1 1] Event when button is pressed, spawns UFOS randomly between 2 and 5 in random locations
  (|CallParentFunction)
  (for _index (range 0 (Math|Random|RandomIntegerinRange 2 5))
    (Game|SpawnActorfromClass "/Game/BP_UFO.BP_UFO_C" (Math|Transform|MakeTransform (Math|Random|RandomPointinBoundingBox (Transformation|GetWorldLocation _box) (Math|Vector|RotateVector (Components|Box|GetScaledBoxExtent _box) (Transformation|GetWorldRotation _box))) "0, 0, 0" "1,1,1") "Undefined" 0 0)))

(fn ConstructionScript
  (|CallParentFunction))