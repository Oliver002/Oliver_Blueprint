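; UFO actor that snaps to hover 150 units above the surface beneath it when play begins.
; UpdateHeight line-traces 300 units down, with debug drawing, and moves the actor to the desired height above the hit.
; A timeline lerps the SUFO component's relative location and rotation for bobbing and turning, though no graph event starts it.
; The construction script sets that timeline's play rate from Speed.
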(event EventBeginPlay
  ;[1 1 1] When Game starts, run this function
  (CallFunction|UpdateHeight 1.5e+02))

(fn ConstructionScript
  (Components|Timeline|SetPlayRate (Variables|Default|GetUFO%20Animation) (Variables|Properties|GetSpeed)))

(fn UpdateHeight
  (params (DesiredHeight :type Float%20%28single-precision%29))
  (bind _returnvalue (Transformation|GetActorLocation))
  ;[1 1 1] Line Trace between UFO loc and Hit loc (300)
  (bind (_outhit _returnvalue_2) (Collision|LineTraceByChannel _returnvalue (- _returnvalue "0, 0,300.000000") "TraceTypeQuery1" false 0 "ForDuration"))
  ;[1 1 1] If Hit == True
  (if _returnvalue_2
    (if (!= (Math|Vector|Distance(Vector) (Transformation|GetActorLocation) (.Location (Collision|BreakHitResult _outhit))) DesiredHeight)
      ;[1 1 1] Set UFO loc on hit loc
      (Transformation|SetActorLocation (+ (.Location (Collision|BreakHitResult _outhit)) (Math|Vector|MakeVector 0.0 0.0 DesiredHeight)) false false))))