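; BP_Button_Reset is a child button Blueprint that resets the scene's UFOs and bombs when pressed.
; After the parent press logic runs, it destroys every BP_UFO and BP_Bomb actor found with GetAllActorsOfClass.
; It then clears and invalidates the spawn timer on the first BP_Button_Spawnbomb found, with no check that one exists.
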(event EventBeginPlay)

(event Collision|EventActorBeginOverlap
  (params (OtherActor :type Actor%20Object%20Reference))
  (|CallParentFunction OtherActor) ; This node is disabled and will not be called.\nDrag off pins to build functionality.
)

(event EventTick
  (params (DeltaSeconds :type Float%20%28single-precision%29)))

(event EventButtonPressed
  (|CallParentFunction)
  ;[0.8503 0 1] Destroy AlL UFOS
  (bind _outactors (Actor|GetAllActorsOfClass "/Game/BP_UFO.BP_UFO_C"))
  (Actor|DestroyActor _outactors)
  ;[1 0 0.03614] Destroy All Bombs
  (bind _outactors_2 (Actor|GetAllActorsOfClass "/Game/BP_Bomb.BP_Bomb_C"))
  (Actor|DestroyActor _outactors_2)
  ;[1 1 1] Clear Bomb Spawn Timer
  (bind _outactors_3 (Actor|GetAllActorsOfClass "/Game/BP_Button_Spawnbomb.BP_Button_Spawnbomb_C"))
  (Utilities|Time|ClearandInvalidateTimerbyHandle (Variables|/Game/BP_Button_Spawnbomb.BP_Button_Spawnbomb_C|GetTimer (Utilities|Array|Get(acopy) _outactors_3))))

(fn ConstructionScript
  (|CallParentFunction))