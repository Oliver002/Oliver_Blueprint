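; A floor button that glows green while a pawn stands on it and turns red when one steps off.
; Actor overlap events filter for Pawns and call the ButtonPressed and ButtonReleased events.
; Each press creates a new dynamic material instance from M_Red on Cylinder1 and sets its Emissive color, which release changes back through the stored instance.
; It only changes color and triggers nothing else.
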(event Custom|Button%20Released
  (bind _button_material (Variables|Default|GetButton%20material))
  ;[1 1 1] When button is released, set it to Red
  (Utilities|IsValid _button_material
    (:Is%20Valid
      (Rendering|Material|SetVectorParameterValue _button_material "Emissive" "(R=1.000000,G=0.000000,B=0.000000,A=1.000000)" :!class /Script/Engine.MaterialInstanceDynamic))))

(event Custom|Button%20Pressed
  ;[1 1 1] When button is pressed, set it to green
  (bind _returnvalue (Rendering|Material|CreateDynamicMaterialInstance (Variables|Default|GetCylinder1) 0 "/Game/M_Red.M_Red" "None" :!class /Script/Engine.PrimitiveComponent))
  (bind _output_get (Variables|Default|SetButton%20material _returnvalue))
  (Rendering|Material|SetVectorParameterValue _output_get "Emissive" "(R=0.000000,G=1.000000,B=0.000000,A=1.000000)" :!class /Script/Engine.MaterialInstanceDynamic))

(event Collision|EventActorBeginOverlap
  (params (OtherActor :type Actor%20Object%20Reference))
  ;[1 1 1] Event that allows the player to stand over the button
  (Utilities|Casting|CastToPawn OtherActor)
  (CallFunction|ButtonPressed))

(event Collision|EventActorEndOverlap
  (params (OtherActor :type Actor%20Object%20Reference))
  ;[1 1 1] Event that allows the player to stand over the button
  (Utilities|Casting|CastToPawn OtherActor)
  (CallFunction|ButtonReleased))

(fn ConstructionScript)