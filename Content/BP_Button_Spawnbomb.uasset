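; Button variant that, once pressed, keeps spawning bombs at random points within a box area.
; The press event runs the parent button logic, then starts a looping two-second timer and stores its handle; nothing here clears it.
; Each tick of that timer spawns a BP_Bomb at a random point around the Box component, using its scaled extent rotated by its world rotation.
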(event Custom|SpawnBomb
  (bind _box (Variables|Default|GetBox))
  ;[1 1 1] Event when button is pressed, spawn a bomb every 2 seconds
  (Game|SpawnActorfromClass "/Game/BP_Bomb.BP_Bomb_C" (Math|Transform|MakeTransform (Math|Random|RandomPointinBoundingBox (Transformation|GetWorldLocation _box) (Math|Vector|RotateVector (Components|Box|GetScaledBoxExtent _box) (Transformation|GetWorldRotation _box))) "0, 0, 0" "1,1,1") "Undefined" 0 0))

(event EventBeginPlay)

(event Collision|EventActorBeginOverlap
  (params (OtherActor :type Actor%20Object%20Reference))
  (|CallParentFunction OtherActor) ; This node is disabled and will not be called.\nDrag off pins to build functionality.
)

(event EventTick
  (params (DeltaSeconds :type Float%20%28single-precision%29)))

(event EventButtonPressed
  ;[1 1 1] Event when button is pressed, spawn a bomb every 2 seconds
  (|CallParentFunction)
  (bind _returnvalue (Utilities|Time|SetTimerbyEvent (delegate Custom|SpawnBomb) 2.0 true))
  (Variables|Default|SetTimer _returnvalue))

(fn ConstructionScript
  (|CallParentFunction))